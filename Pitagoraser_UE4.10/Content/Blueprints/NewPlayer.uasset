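; Player actor for a domino-placing game, moved forward and back along its control yaw (unless disabled) and turned by the side axis.
; Once the tutorial step in dominoInstance reaches seven, stick input sets flags there.
; Overlaps with Domino-tagged actors toggle that instance's Setting flag and reset its SetTime on exit to prevent consecutive placement.
; Tick accumulates SetTime and locks height to the starting Z.
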(event Collision|EventActorBeginOverlap
  (params (OtherActor :type Actor%20Object%20Reference))
  ;[1 1 1] 連続でドミノを置けないように
  (if (Actor|ActorHasTag OtherActor "Domino")
    (bind _asdomino_instance (Utilities|Casting|CastTodominoInstance (Game|GetGameInstance)))
    (Variables|/Game/Blueprints/dominoInstance.dominoInstance_C|SetSetting _asdomino_instance false)))

(event Collision|EventActorEndOverlap
  (params (OtherActor :type Actor%20Object%20Reference))
  ;[1 1 1] 連続でドミノを置けないように
  (if (Actor|ActorHasTag OtherActor "Domino")
    (bind _asdomino_instance (Utilities|Casting|CastTodominoInstance (Game|GetGameInstance)))
    (Variables|/Game/Blueprints/dominoInstance.dominoInstance_C|SetSetting _asdomino_instance true)
    (Variables|/Game/Blueprints/dominoInstance.dominoInstance_C|SetSetTime _asdomino_instance 0.0)))

(event EventTick
  (params (DeltaSeconds :type Float%20%28single-precision%29))
  (bind _returnvalue (Transformation|GetActorLocation))
  (bind _defaultz (Variables|Default|GetDefaultZ))
  ;[1 1 1] Tick
  (bind _asdomino_instance (Utilities|Casting|CastTodominoInstance (Game|GetGameInstance)))
  (Variables|/Game/Blueprints/dominoInstance.dominoInstance_C|SetSetTime _asdomino_instance (+ DeltaSeconds (Variables|/Game/Blueprints/dominoInstance.dominoInstance_C|GetSetTime _asdomino_instance)))
  (if (!= (.z _returnvalue) _defaultz)
    (Transformation|SetActorLocation (Math|Vector|MakeVector (.x _returnvalue) (.y _returnvalue) _defaultz) false false)))

(event EventBeginPlay
  (Variables|Default|SetDefaultZ (.z (Transformation|GetActorLocation))))

(event Input|AxisEvents|InputAxisMoveForward
  (params (AxisValue :type Float%20%28single-precision%29))
  ;[1 1 1] Move
  (if (not (Variables|Default|GetDisable))
    (Pawn|Input|AddMovementInput (Math|Vector|GetForwardVector (Math|Rotator|MakeRotator 0.0 0.0 (.Yaw (Math|Rotator|BreakRotator (Pawn|GetControlRotation :!class /Script/Engine.Pawn))))) AxisValue false)
    (if (!= AxisValue 0.0)
      (bind _asdomino_instance (Utilities|Casting|CastTodominoInstance (Game|GetGameInstance)))
      (if (>= (Variables|/Game/Blueprints/dominoInstance.dominoInstance_C|GetTyutoNum _asdomino_instance) 7)
        (Variables|/Game/Blueprints/dominoInstance.dominoInstance_C|SetRightStickUpDown _asdomino_instance true)))))

(event Input|AxisEvents|InputAxisMoveSide
  (params (AxisValue :type Float%20%28single-precision%29))
  ;[1 1 1] Rotation
  (Pawn|Input|AddControllerYawInput AxisValue)
  (bind _asdomino_instance (Utilities|Casting|CastTodominoInstance (Game|GetGameInstance)))
  (if (>= (Variables|/Game/Blueprints/dominoInstance.dominoInstance_C|GetTyutoNum _asdomino_instance) 7)
    (if (!= AxisValue 0.0)
      (Variables|/Game/Blueprints/dominoInstance.dominoInstance_C|SetRightStickLR _asdomino_instance true))))

(fn ConstructionScript)
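; BooksBP is a gimmick prop, apparently books, that returns to its starting placement after a domino knocks into it.
; It stores its transform at BeginPlay and sets a Clash flag when hit by an actor tagged Domino.
; While the flag is set, Tick accumulates time, then after about 15 seconds restores the stored transform without sweep and clears the flag and timer.
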(event EventHit
  (params (MyComp :type Primitive%20Component%20Object%20Reference) (Other :type Actor%20Object%20Reference) (OtherComp :type Primitive%20Component%20Object%20Reference) (bSelfMoved :type Boolean) (HitLocation :type Vector :default "0, 0, 0") (HitNormal :type Vector :default "0, 0, 0") (NormalImpulse :type Vector :default "0, 0, 0") (Hit :type Hit%20Result%20Structure%20%28by%20ref%29))
  (if (Actor|ActorHasTag Other "Domino")
    (Variables|Default|SetClash true)))

(event EventBeginPlay
  (Variables|Default|SetOriginTransform (Transformation|GetActorTransform)))

(event EventTick
  (params (DeltaSeconds :type Float%20%28single-precision%29))
  (if (Variables|Default|GetClash)
    (Variables|Default|Settime (+ DeltaSeconds (Variables|Default|Gettime)))
    (if (and (> (+ DeltaSeconds (Variables|Default|Gettime)) 15.0) (Variables|Default|GetClash))
      (Transformation|SetActorTransform (Variables|Default|GetOriginTransform))
      (Variables|Default|SetClash false)
      (Variables|Default|SetTime 0.0))))

(fn ConstructionScript)
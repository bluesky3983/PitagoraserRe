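; pitaGameState is, by its name, a game state Blueprint that serves as a shared store for gameplay values.
; It exposes plain getter and setter functions for CakeHit, PlayerHp, Radial and StartUI, with each setter returning the stored value.
; It has no logic of its own: BeginPlay, Tick and the construction script are empty, so other code must drive these values.
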(event EventBeginPlay)

(event EventTick
  (params (DeltaSeconds :type Float%20%28single-precision%29)))

(fn ConstructionScript)

(fn GetCakeHit
  (return (Variables|Default|GetCakeHit)))

(fn GetPlayerHp
  (return (Variables|Default|GetPlayerHp)))

(fn GetRadial
  (return (Variables|Default|Getradial)))

(fn GetStartUI
  (return (Variables|Default|GetStartUI)))

(fn SetCakeHit
  (params (NewParam :type Boolean))
  (bind _output_get (Variables|Default|SetCakeHit NewParam))
  (return _output_get))

(fn SetPlayerHp
  (params (NewParam :type Integer))
  (bind _output_get (Variables|Default|SetPlayerHp NewParam))
  (return _output_get))

(fn SetRadial
  (params (NewParam1 :type Radial%20Force%20Component%20Object%20Reference))
  (bind _output_get (Variables|Default|Setradial NewParam1))
  (return _output_get))

(fn SetStartUI
  (params (NewParam :type Integer))
  (bind _output_get (Variables|Default|SetStartUI NewParam))
  (return _output_get))
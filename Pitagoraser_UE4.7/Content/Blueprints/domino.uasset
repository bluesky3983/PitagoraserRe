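; Domino actor that detects being knocked by another domino and removes itself afterwards.
; Its first hit from an actor tagged "Domino" adds an entry to the game instance's ClashDomino array, sets a clashed flag and plays a falling sound at world origin.
; Tick then accumulates time and destroys the actor after roughly ten seconds.
; BeginPlay also calls SetRadialMessage on the game state.
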(event EventHit
  (params (MyComp :type Primitive%20Component%20Object%20Reference) (Other :type Actor%20Object%20Reference) (OtherComp :type Primitive%20Component%20Object%20Reference) (bSelfMoved :type Boolean) (HitLocation :type Vector :default "0, 0, 0") (HitNormal :type Vector :default "0, 0, 0") (NormalImpulse :type Vector :default "0, 0, 0") (Hit :type Hit%20Result%20Structure%20%28by%20ref%29))
  (if (Actor|ActorHasTag Other "Domino")
    (Utilities|FlowControl|DoOnce false
      (:Completed
        (bind _asdomino_instance (Utilities|Casting|CastTodominoInstance (Game|GetGameInstance)))
        (Utilities|Array|Add (Variables|/Game/Blueprints/dominoInstance.dominoInstance_C|GetClashDomino _asdomino_instance) 0)
        (Variables|Default|SetClashed true)
        (Audio|PlaySoundatLocation "/Game/Sound/domino_down2.domino_down2" "0, 0, 0")))))

(event EventBeginPlay
  (Class|Pita|SetRadial(Message) (Game|GetGameState)))

(event EventTick
  (params (DeltaSeconds :type Float%20%28single-precision%29))
  (if (Variables|Default|GetClashed)
    (Variables|Default|Settime (+ DeltaSeconds (Variables|Default|Gettime)))
    (if (and (> (+ DeltaSeconds (Variables|Default|Gettime)) 1e+01) (Variables|Default|GetClashed))
      (Actor|DestroyActor))))

(fn ConstructionScript)